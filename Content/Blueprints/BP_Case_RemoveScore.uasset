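; BP_Case_RemoveScore is a tabletop board space, going by its name, whose action subtracts points from a player's score.
; Its Action override calls the parent, then casts the game instance to GI_Tabletop and sets that player's score, by player number, to the current score minus ScoreValue.
; It prints the new score on screen; the event graph is otherwise unused.
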(event EventBeginPlay
  (|CallParentFunction) ; This node is disabled and will not be called.\nDrag off pins to build functionality.
)

(event Collision|EventActorBeginOverlap
  (params (OtherActor :type Actor%20Object%20Reference))
  (|CallParentFunction OtherActor) ; This node is disabled and will not be called.\nDrag off pins to build functionality.
)

(event EventTick
  (params (DeltaSeconds :type Float%20%28single-precision%29))
  (|CallParentFunction DeltaSeconds) ; This node is disabled and will not be called.\nDrag off pins to build functionality.
)

(fn ConstructionScript
  (|CallParentFunction))

(fn Action
  (params (PlayerStruct :type Struct%20Player%20Structure))
  (bind (_playernumber _score) (Utilities|Struct|BreakStruct_Player PlayerStruct))
  (bind _scorevalue (Variables|Default|GetScoreValue))
  (bind _returnvalue (- _score _scorevalue))
  (|CallParentFunction PlayerStruct)
  (bind _asgi_tabletop (Utilities|Casting|CastToGI_Tabletop (Game|GetGameInstance)))
  (Default|SetPlayerScorebyPlayerId _asgi_tabletop _playernumber _returnvalue)
  (Development|PrintString (Utilities|String|Append "New score is : " (Utilities|String|ToString(Integer) _returnvalue))))