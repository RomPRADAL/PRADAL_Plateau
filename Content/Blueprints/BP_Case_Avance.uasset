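; BP_Case_Avance is a tabletop board cell ("case avance") that moves the player's pawn along the grid by an offset.
; Its Action override calls the parent, finds its own index in the GM_Tabletop grid and adds ValeurDeDeplacement.
; If that index is non-negative (no upper bound check), the pawn moves to the target cell's first available slot.
; Debug strings report success or failure.
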(event EventBeginPlay
  (|CallParentFunction) ; This node is disabled and will not be called.\nDrag off pins to build functionality.
)

(event Collision|EventActorBeginOverlap
  (params (OtherActor :type Actor%20Object%20Reference))
  (|CallParentFunction OtherActor) ; This node is disabled and will not be called.\nDrag off pins to build functionality.
)

(event EventTick
  (params (DeltaSeconds :type Float%20%28single-precision%29))
  (|CallParentFunction DeltaSeconds) ; This node is disabled and will not be called.\nDrag off pins to build functionality.
)

(fn ConstructionScript
  (|CallParentFunction))

(fn Action
  (params (PlayerStruct :type Struct%20Player%20Structure))
  (|CallParentFunction (Utilities|Struct|MakeStruct_Player (.playernumber PlayerStruct) (.score PlayerStruct) (.position PlayerStruct) (.playerinlevel PlayerStruct)))
  (bind _asgm_tabletop (Utilities|Casting|CastToGM_Tabletop (Game|GetGameMode)))
  (if (>= (+ (Utilities|Array|FindItem (Variables|/Game/Blueprints/BP_Grid.BP_Grid_C|GetGrid (Variables|/Game/Blueprints/GM_Tabletop.GM_Tabletop_C|GetGridRef _asgm_tabletop)) self) (Variables|Default|GetValeurDeDeplacement)) 0)
    (bind _couldmove (Default|MovePiontoFirstSlotAvailableinCell (.playerinlevel PlayerStruct) (Utilities|Array|Get(acopy) (Variables|/Game/Blueprints/BP_Grid.BP_Grid_C|GetGrid (Variables|/Game/Blueprints/GM_Tabletop.GM_Tabletop_C|GetGridRef _asgm_tabletop)) (+ (Utilities|Array|FindItem (Variables|/Game/Blueprints/BP_Grid.BP_Grid_C|GetGrid (Variables|/Game/Blueprints/GM_Tabletop.GM_Tabletop_C|GetGridRef _asgm_tabletop)) self) (Variables|Default|GetValeurDeDeplacement)))))
    (if _couldmove
      (Development|PrintString "On a avancé !")
      (else
        (Development|PrintString "Could not move")))
    (else
      (Development|PrintString "Peut pas avancer"))))