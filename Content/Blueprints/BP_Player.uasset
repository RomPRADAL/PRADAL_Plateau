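; BP_Player represents a board game player that moves its piece, PlayerPion, between the slots of board cells.
; MovePionToFirstSlotAvailableInCell asks a Cell for an available slot, fills it, then passes that slot's position to MovePionVector.
; MovePionVector sets the piece's root world location directly without sweep, and a full cell makes the move report failure.
; The event graph and construction script are empty, so it only acts when called.
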(event EventBeginPlay)

(event Collision|EventActorBeginOverlap
  (params (OtherActor :type Actor%20Object%20Reference)))

(event EventTick
  (params (DeltaSeconds :type Float%20%28single-precision%29)))

(fn ConstructionScript)

(fn MovePionVector
  (params (VectorToMoveTo :type Vector))
  (Transformation|SetWorldLocation (Variables|/Game/Blueprints/BP_GoodPion.BP_GoodPion_C|GetDefaultSceneRoot (Variables|Default|GetPlayerPion)) VectorToMoveTo false false))

(fn MovePiontoFirstSlotAvailableinCell
  (params (Cell :type BP%20Case%20Object%20Reference))
  ;[1 0.7952 0.01201] Sainte Trinité du Move
  (bind (_indexslot _isfull) (Default|GetAvailableSlot Cell))
  (if (not _isfull)
    (Default|FillSlot Cell _indexslot)
    (bind _position (Default|GetSlotPosition Cell _indexslot))
    (CallFunction|MovePionVector _position)
    (else
      (LocalVariables|SetRetCouldMove false)))
  (return (LocalVariables|GetRetCouldMove)))