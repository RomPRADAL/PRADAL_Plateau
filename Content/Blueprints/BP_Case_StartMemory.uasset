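; Board case Blueprint for the tabletop game that starts the memory minigame.
; Its Action override runs the parent logic, then uses the GM_Tabletop game mode to move the camera to the memory board and initialize the memory cases through its MemoryRef.
; A debug string prints on start, and the event graph holds only disabled default events.
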(event EventBeginPlay
  (|CallParentFunction) ; This node is disabled and will not be called.\nDrag off pins to build functionality.
)

(event Collision|EventActorBeginOverlap
  (params (OtherActor :type Actor%20Object%20Reference))
  (|CallParentFunction OtherActor) ; This node is disabled and will not be called.\nDrag off pins to build functionality.
)

(event EventTick
  (params (DeltaSeconds :type Float%20%28single-precision%29))
  (|CallParentFunction DeltaSeconds) ; This node is disabled and will not be called.\nDrag off pins to build functionality.
)

(fn ConstructionScript
  (|CallParentFunction))

(fn Action
  (params (PlayerStruct :type Struct%20Player%20Structure))
  (|CallParentFunction PlayerStruct)
  (bind _asgm_tabletop (Utilities|Casting|CastToGM_Tabletop (Game|GetGameMode)))
  (Default|MoveCameratoMemory _asgm_tabletop)
  (Development|PrintString "Start memory")
  (Default|InitMemoryCases (Variables|/Game/Blueprints/GM_Tabletop.GM_Tabletop_C|GetMemoryRef _asgm_tabletop)))