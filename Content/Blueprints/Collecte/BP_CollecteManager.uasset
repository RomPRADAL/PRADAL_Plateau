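; Manager for collectable items in a tabletop game, which also awards score on a win.
; On BeginPlay it caches every Collectable actor in the level into CollectablesList.
; WinScoreAction adds points in the game instance's PlayerList to the player opposite TurnPlayerIndex, handling two players only.
; It then refreshes the score display through the game mode's InfoRef.
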(event EventBeginPlay
  (bind _outactors (Actor|GetAllActorsOfClass "/Script/SuperJeuDeLoie.Collectable"))
  (Variables|Default|SetCollectablesList _outactors))

(event EventWinScoreAction
  (bind _asgi_tabletop (Utilities|Casting|CastToGI_Tabletop (Game|GetGameInstance)))
  (switch int (Variables|/Game/Blueprints/GI_Tabletop.GI_Tabletop_C|GetTurnPlayerIndex _asgi_tabletop)
    (:0
      (Utilities|Array|SetArrayElem (Variables|/Game/Blueprints/GI_Tabletop.GI_Tabletop_C|GetPlayerList _asgi_tabletop) 1 (Utilities|Struct|MakeStruct_Player (.playernumber (Utilities|Array|Get(acopy) (Variables|/Game/Blueprints/GI_Tabletop.GI_Tabletop_C|GetPlayerList _asgi_tabletop) 1)) (+ (.score (Utilities|Array|Get(acopy) (Variables|/Game/Blueprints/GI_Tabletop.GI_Tabletop_C|GetPlayerList _asgi_tabletop) 1)) 2) (.position (Utilities|Array|Get(acopy) (Variables|/Game/Blueprints/GI_Tabletop.GI_Tabletop_C|GetPlayerList _asgi_tabletop) 1)) (.playerinlevel (Utilities|Array|Get(acopy) (Variables|/Game/Blueprints/GI_Tabletop.GI_Tabletop_C|GetPlayerList _asgi_tabletop) 1)))))
    (:1
      (Utilities|Array|SetArrayElem (Variables|/Game/Blueprints/GI_Tabletop.GI_Tabletop_C|GetPlayerList _asgi_tabletop) 0 (Utilities|Struct|MakeStruct_Player (.playernumber (Utilities|Array|Get(acopy) (Variables|/Game/Blueprints/GI_Tabletop.GI_Tabletop_C|GetPlayerList _asgi_tabletop))) (+ (.score (Utilities|Array|Get(acopy) (Variables|/Game/Blueprints/GI_Tabletop.GI_Tabletop_C|GetPlayerList _asgi_tabletop))) 2) (.position (Utilities|Array|Get(acopy) (Variables|/Game/Blueprints/GI_Tabletop.GI_Tabletop_C|GetPlayerList _asgi_tabletop))) (.playerinlevel (Utilities|Array|Get(acopy) (Variables|/Game/Blueprints/GI_Tabletop.GI_Tabletop_C|GetPlayerList _asgi_tabletop)))))))
  (bind _asgm_tabletop (Utilities|Casting|CastToGM_Tabletop (Game|GetGameMode)))
  (Default|UpdateScore (Variables|/Game/Blueprints/GM_Tabletop.GM_Tabletop_C|GetInfoRef _asgm_tabletop)))

(fn ConstructionScript)