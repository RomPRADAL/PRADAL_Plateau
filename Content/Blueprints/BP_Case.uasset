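; BP_Case is an actor that manages a set of positioned slots, each either free or occupied.
; GetAvailableSlot returns the first free index, but its IsFull check never triggers, so a full case yields index 0.
; FillSlot and ClearSlot toggle a slot's Free flag while keeping its position.
; GetSlotPosition adds the actor location to the stored offset, ignoring rotation and scale.
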(event EventBeginPlay)

(event Collision|EventActorBeginOverlap
  (params (OtherActor :type Actor%20Object%20Reference)))

(event EventTick
  (params (DeltaSeconds :type Float%20%28single-precision%29)))

(fn ConstructionScript)

(fn GetAvailableSlot
  ;[0.5979 0.156 1] Pas Necessaire mais on est jamais trop prudent
  (LocalVariables|SetRetIsFull false)
  (LocalVariables|SetRetIndexSlot 0)
  (bind (_array_element _array_index) (Utilities|Array|ForEachLoopwithBreak (Variables|Default|GetSlots) :!label _label)
    (:LoopBody
      (if (.Free (Utilities|Struct|BreakStruct_Slot _array_element))
        (LocalVariables|SetRetIndexSlot _array_index)
        (goto _label Break)))
    (:Completed
      (if (> (LocalVariables|GetRetIndexSlot) (Utilities|Array|Length (Variables|Default|GetSlots)))
        (LocalVariables|SetRetIsFull true))
      (return (LocalVariables|GetRetIndexSlot) (LocalVariables|GetRetIsFull)))))

(fn FillSlot
  (params (SlotIndex :type Integer))
  (bind _slots (Variables|Default|GetSlots))
  (Utilities|Array|SetArrayElem _slots SlotIndex (Utilities|Struct|MakeStruct_Slot false (.Position (Utilities|Struct|BreakStruct_Slot (Utilities|Array|Get(acopy) _slots SlotIndex))))))

(fn ClearSlot
  (params (SlotIndex :type Integer))
  (bind _slots (Variables|Default|GetSlots))
  (Utilities|Array|SetArrayElem _slots SlotIndex (Utilities|Struct|MakeStruct_Slot true (.Position (Utilities|Struct|BreakStruct_Slot (Utilities|Array|Get(acopy) _slots SlotIndex))))))

(fn GetSlotPosition
  (params (SlotIndex :type Integer))
  (return (+ (.position (Utilities|Array|Get(acopy) (Variables|Default|GetSlots) SlotIndex)) (Transformation|GetActorLocation))))