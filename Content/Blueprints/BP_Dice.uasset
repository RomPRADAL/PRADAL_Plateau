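; BP_Dice is a dice-rolling Blueprint that produces random results within a configurable value range.
; RollDice returns a random integer between ValueMin and ValueMax, and RollMultipleDice calls it repeatedly to return the summed total.
; ChangeDiceValue updates the range at runtime, and both roll functions print their results on screen for debugging.
; The event graph and construction script are empty, so rolls happen only when other code calls these functions.
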(event EventBeginPlay)

(event Collision|EventActorBeginOverlap
  (params (OtherActor :type Actor%20Object%20Reference)))

(event EventTick
  (params (DeltaSeconds :type Float%20%28single-precision%29)))

(fn ConstructionScript)

(fn RollDice
  (bind _output_get (LocalVariables|SetDiceResult (Math|Random|RandomIntegerinRange (Variables|Default|GetValueMin) (Variables|Default|GetValueMax))))
  (Development|PrintString (Utilities|String|Append "Dice Result : " (Utilities|String|ToString(Integer) _output_get)) true true "(R=0.000000,G=1.000000,B=0.300213,A=1.000000)" 1e+01)
  (return _output_get))

(fn RollMultipleDice
  (params (NumberOfDice :type Integer))
  (LocalVariables|SetAllDicesResult 0)
  (for _index (range 1 NumberOfDice)
    (bind _result (CallFunction|RollDice))
    (LocalVariables|SetAllDicesResult (+ (LocalVariables|GetAllDicesResult) _result))
    (Development|PrintString (Utilities|String|Append "Dice " (Utilities|String|ToString(Integer) _index) ": " (Utilities|String|ToString(Integer) _result))))
  (Development|PrintString (Utilities|String|Append "All Dices result" (Utilities|String|ToString(Integer) (LocalVariables|GetAllDicesResult))) true true "(R=0.000000,G=0.301191,B=1.000000,A=1.000000)" 5.0)
  (return (LocalVariables|GetAllDicesResult)))

(fn ChangeDiceValue
  (params (NewMin :type Integer) (NewMax :type Integer))
  (Variables|Default|SetValueMin NewMin)
  (Variables|Default|SetValueMax NewMax))