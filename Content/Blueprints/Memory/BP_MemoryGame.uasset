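; Manager for the memory pair-matching minigame in the tabletop game, shuffling all BP_MemoryCase actors into pairs.
; WaitThenHide freezes input for a timed comparison: matches deactivate and score, misses hide and cost an attempt.
; Winning adds points to the PlayerList entry opposite TurnPlayerIndex in GI_Tabletop.
; GM_Tabletop updates the memory UI and, on win or loss, returns the camera to the board while the game resets.
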(event Custom|WaitThenHide
  (CallFunction|FreezeGame)
  (Utilities|Time|SetTimerbyEvent (delegate Custom|CheckPairThenHide) 2.0))

(event Custom|CheckPairThenHide
  (bind _pairetrouvé_ (CallFunction|CompareRevealedCases))
  (if _pairetrouvé_
    _
    (else
      (CallFunction|LowerTentatives)
      (CallFunction|HideRevealedCases)))
  (CallFunction|UnfreezeGame))

(event EventBeginPlay
  (Utilities|FlowControl|Sequence
    (:then_0
      (bind _outactors (Actor|GetAllActorsOfClass "/Game/Blueprints/Memory/BP_MemoryCase.BP_MemoryCase_C"))
      (Variables|Default|SetAllMemoryCases _outactors))
    (:then_1
      (CallFunction|InitMemoryCases))))

(fn ConstructionScript)

(fn CompareRevealedCases
  (if (and (Utilities|IsValid (Variables|Default|GetFirstCaseRevealed)) (Utilities|IsValid (Variables|Default|GetSecondCaseRevealed)))
    (if (== (Variables|/Game/Blueprints/Memory/BP_MemoryCase.BP_MemoryCase_C|GetPair (Variables|Default|GetFirstCaseRevealed)) (Variables|/Game/Blueprints/Memory/BP_MemoryCase.BP_MemoryCase_C|GetPair (Variables|Default|GetSecondCaseRevealed)))
      (CallFunction|DesactivateRevealedCases)
      (CallFunction|UpMemoryScore)
      (LocalVariables|SetRetPaireTrouvé true))
    (return (LocalVariables|GetRetPaireTrouvé))
    (else
      (Development|PrintString "(COMPARE) Une case est invalide"))))

(fn HideRevealedCases
  (if (and (Utilities|IsValid (Variables|Default|GetFirstCaseRevealed)) (Utilities|IsValid (Variables|Default|GetSecondCaseRevealed)))
    (Default|Hide (Variables|Default|GetFirstCaseRevealed))
    (else
      (Development|PrintString "(HIDE) Une case est invalide"))))

(fn DesactivateRevealedCases
  (if (and (Utilities|IsValid (Variables|Default|GetFirstCaseRevealed)) (Utilities|IsValid (Variables|Default|GetSecondCaseRevealed)))
    (Default|Desactivate (Variables|Default|GetFirstCaseRevealed))
    (else
      (Development|PrintString "(DESACTIVATE) Une case est invalide"))))

(fn InitMemoryCases
  (bind _allmemorycases (Variables|Default|GetAllMemoryCases))
  (Utilities|FlowControl|Sequence
    (:then_0
      (Utilities|Array|Shuffle _allmemorycases)
      (for (_array_element _array_index) _allmemorycases
        (Variables|/Game/Blueprints/Memory/BP_MemoryCase.BP_MemoryCase_C|SetPair _array_element (LocalVariables|GetSuperInteger))
        (Default|InitMaterialReveal _array_element)
        (if (== (Math|Integer|%(Integer) _array_index 2) 1)
          (Math|Integer|IncrementInt (LocalVariables|GetSuperInteger)))))
    (:then_1
      (for _array_element_2 (Variables|Default|GetAllMemoryCases)
        (Default|Hide _array_element_2)
        (Variables|/Game/Blueprints/Memory/BP_MemoryCase.BP_MemoryCase_C|SetActive _array_element_2 true)))
    (:then_2
      (Variables|Default|SetGameFreeze false)
      (Variables|Default|SetScore 0)
      (Variables|Default|SetNumberRevealed 0)
      (Variables|Default|SetNumbreDeCoups 10)
      (Variables|Default|SetTentatives 10)
      (Variables|Default|SetFirstCaseRevealed 0)
      (Variables|Default|SetSecondCaseRevealed 0))))

(fn FreezeGame
  (Variables|Default|SetGameFreeze true))

(fn UnfreezeGame
  (Variables|Default|SetGameFreeze false))

(fn UpMemoryScore
  (Math|Integer|IncrementInt (Variables|Default|GetScore)
    (:%20%20
      (bind _asgm_tabletop (Utilities|Casting|CastToGM_Tabletop (Game|GetGameMode)))
      (Default|UpdateScore (Variables|/Game/Blueprints/GM_Tabletop.GM_Tabletop_C|GetInfoMemoryRef _asgm_tabletop) (Variables|Default|GetScore))
      (CallFunction|CheckWinLoose))))

(fn CheckWinLoose
  (if (>= (Variables|Default|GetScore) 8)
    (Utilities|FlowControl|Sequence
      (:then_0
        (bind _asgi_tabletop (Utilities|Casting|CastToGI_Tabletop (Game|GetGameInstance)))
        (switch int (Variables|/Game/Blueprints/GI_Tabletop.GI_Tabletop_C|GetTurnPlayerIndex _asgi_tabletop)
          (:0
            (Utilities|Array|SetArrayElem (Variables|/Game/Blueprints/GI_Tabletop.GI_Tabletop_C|GetPlayerList _asgi_tabletop) 1 (Utilities|Struct|MakeStruct_Player (.playernumber (Utilities|Array|Get(acopy) (Variables|/Game/Blueprints/GI_Tabletop.GI_Tabletop_C|GetPlayerList _asgi_tabletop) 1)) (+ (.score (Utilities|Array|Get(acopy) (Variables|/Game/Blueprints/GI_Tabletop.GI_Tabletop_C|GetPlayerList _asgi_tabletop) 1)) 2) (.position (Utilities|Array|Get(acopy) (Variables|/Game/Blueprints/GI_Tabletop.GI_Tabletop_C|GetPlayerList _asgi_tabletop) 1)) (.playerinlevel (Utilities|Array|Get(acopy) (Variables|/Game/Blueprints/GI_Tabletop.GI_Tabletop_C|GetPlayerList _asgi_tabletop) 1)))))
          (:1
            (Utilities|Array|SetArrayElem (Variables|/Game/Blueprints/GI_Tabletop.GI_Tabletop_C|GetPlayerList _asgi_tabletop) 0 (Utilities|Struct|MakeStruct_Player (.playernumber (Utilities|Array|Get(acopy) (Variables|/Game/Blueprints/GI_Tabletop.GI_Tabletop_C|GetPlayerList _asgi_tabletop))) (+ (.score (Utilities|Array|Get(acopy) (Variables|/Game/Blueprints/GI_Tabletop.GI_Tabletop_C|GetPlayerList _asgi_tabletop))) 2) (.position (Utilities|Array|Get(acopy) (Variables|/Game/Blueprints/GI_Tabletop.GI_Tabletop_C|GetPlayerList _asgi_tabletop))) (.playerinlevel (Utilities|Array|Get(acopy) (Variables|/Game/Blueprints/GI_Tabletop.GI_Tabletop_C|GetPlayerList _asgi_tabletop)))))))
        (CallFunction|InitMemoryCases)
        (for (_array_element _array_index) (Variables|/Game/Blueprints/GI_Tabletop.GI_Tabletop_C|GetPlayerList _asgi_tabletop)
          (Development|PrintString (Utilities|String|Append (Utilities|String|ToString(Integer) (.playernumber _array_element)) " " (Utilities|String|ToString(Integer) (.score _array_element)) " " (Utilities|String|ToString(Integer) (.position _array_element)) " " (Utilities|GetDisplayName (.playerinlevel _array_element)) " " (Utilities|String|ToString(Integer) _array_index)) true true "(R=0.000000,G=0.660000,B=1.000000,A=1.000000)" 1e+01)))
      (:then_1
        (bind _asgm_tabletop (Utilities|Casting|CastToGM_Tabletop (Game|GetGameMode)))
        (Default|MoveCameratoBoard _asgm_tabletop)
        (Default|ShowInfoWidget _asgm_tabletop)))
    (elif (<= (Variables|Default|GetTentatives) 0)
      (bind _asgm_tabletop_2 (Utilities|Casting|CastToGM_Tabletop (Game|GetGameMode)))
      (Default|MoveCameratoBoard _asgm_tabletop_2)
      (Default|ShowInfoWidget _asgm_tabletop_2)
      (CallFunction|InitMemoryCases))))

(fn LowerTentatives
  (bind _result (Math|Integer|DecrementInt (Variables|Default|GetTentatives))
    (:%20%20
      (bind _asgm_tabletop (Utilities|Casting|CastToGM_Tabletop (Game|GetGameMode)))
      (Default|UpdateTentative (Variables|/Game/Blueprints/GM_Tabletop.GM_Tabletop_C|GetInfoMemoryRef _asgm_tabletop) _result)
      (CallFunction|CheckWinLoose))))