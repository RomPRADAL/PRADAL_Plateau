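; BP_MemoryCase is a clickable tile in a memory matching game.
; On BeginPlay it finds BP_MemoryGame and picks a colored reveal material from its Pair index.
; A click, allowed when the game is not frozen and the tile is active, reveals it and registers it as first or second pick.
; On the second pick it resets the count and calls the manager's WaitThenHide.
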(event EventBeginPlay
  (Utilities|FlowControl|Delay 0.2)
  (bind _returnvalue (Actor|GetActorOfClass "/Game/Blueprints/Memory/BP_MemoryGame.BP_MemoryGame_C"))
  (Variables|Default|SetMemoryGameRef _returnvalue)
  (switch int (Variables|Default|GetPair)
    (:0
      (Variables|Default|SetMaterialReveal "/Game/Blueprints/Memory/MI_MemoryBlue.MI_MemoryBlue"))
    (:1
      (Variables|Default|SetMaterialReveal "/Game/Blueprints/Memory/MI_MemoryGreen.MI_MemoryGreen"))
    (:2
      (Variables|Default|SetMaterialReveal "/Game/Blueprints/Memory/MI_MemoryOrange.MI_MemoryOrange"))
    (:3
      (Variables|Default|SetMaterialReveal "/Game/Blueprints/Memory/MI_MemoryPink.MI_MemoryPink"))
    (:4
      (Variables|Default|SetMaterialReveal "/Game/Blueprints/Memory/Mi_MemoryRed.Mi_MemoryRed"))
    (:5
      (Variables|Default|SetMaterialReveal "/Game/Blueprints/Memory/MI_MemoryYellow.MI_MemoryYellow"))
    (:6
      (Variables|Default|SetMaterialReveal "/Game/Blueprints/Memory/Mi_memoryCyan.Mi_memoryCyan"))
    (:7
      (Variables|Default|SetMaterialReveal "/Game/Blueprints/Memory/MI_MemoryWhite.MI_MemoryWhite"))))

(event MouseInput|EventActorOnClicked
  (params (ButtonPressed :type Key%20Structure :default "None"))
  (bind _self self)
  (bind _memorygameref (Variables|Default|GetMemoryGameRef))
  (bind _memorygameref_2 (Variables|Default|GetMemoryGameRef))
  (if (not (Variables|/Game/Blueprints/Memory/BP_MemoryGame.BP_MemoryGame_C|GetGameFreeze (Variables|Default|GetMemoryGameRef)))
    (if (and (Variables|Default|GetActive) (not (Variables|Default|GetRevealed)))
      (Development|PrintString "Je reveal")
      (Utilities|FlowControl|Sequence
        (:then_0
          (CallFunction|Reveal)
          (if (== (Variables|/Game/Blueprints/Memory/BP_MemoryGame.BP_MemoryGame_C|GetNumberRevealed _memorygameref) 0)
            (Variables|/Game/Blueprints/Memory/BP_MemoryGame.BP_MemoryGame_C|SetFirstCaseRevealed _memorygameref _self)
            (else
              (Variables|/Game/Blueprints/Memory/BP_MemoryGame.BP_MemoryGame_C|SetSecondCaseRevealed _memorygameref _self)))
          (Math|Integer|IncrementInt (Variables|/Game/Blueprints/Memory/BP_MemoryGame.BP_MemoryGame_C|GetNumberRevealed _memorygameref)))
        (:then_1
          (if (>= (Variables|/Game/Blueprints/Memory/BP_MemoryGame.BP_MemoryGame_C|GetNumberRevealed _memorygameref_2) 2)
            (Development|PrintString "Deux cases tournés")
            (Variables|/Game/Blueprints/Memory/BP_MemoryGame.BP_MemoryGame_C|SetNumberRevealed _memorygameref_2 0)
            (Default|WaitThenHide (Variables|Default|GetMemoryGameRef))))))))

(fn ConstructionScript)

(fn Reveal
  (Variables|Default|SetRevealed true)
  (Rendering|Material|SetMaterial (Variables|Default|GetStaticMesh) 0 (Variables|Default|GetMaterialReveal)))

(fn Hide
  (Variables|Default|SetRevealed false)
  (Rendering|Material|SetMaterial (Variables|Default|GetStaticMesh) 0 (Variables|Default|GetMaterialBase)))

(fn Desactivate
  (Variables|Default|SetActive false))