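; Game mode for a two-player tabletop board game with memory and collect minigames.
; On BeginPlay it spawns the dice, plus a player and pawn piece per GameInstance PlayerList entry, placed on the grid.
; Dice rolls move the current player's piece, alternate turns and show a win widget at the last cell.
; Helper functions switch camera positions, HUD widgets and possession between board and collect pawns.
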(event Custom|ChangeTurn
  (bind _giref (Variables|Default|GetGiRef))
  (bind _inforef (Variables|Default|GetInfoRef))
  ;[0.2891 0.3467 1] Aurait très bien pu être une fonction mais il faut varier un peu
  (if (== (Variables|/Game/Blueprints/GI_Tabletop.GI_Tabletop_C|GetTurnPlayerIndex _giref) 0)
    (Variables|/Game/Blueprints/GI_Tabletop.GI_Tabletop_C|SetTurnPlayerIndex _giref 1)
    (Default|ChangeTextTurn _inforef "Tour du joueur : Joueur 2")
    (else
      (Variables|/Game/Blueprints/GI_Tabletop.GI_Tabletop_C|SetTurnPlayerIndex _giref 0)
      (Default|ChangeTextTurn _inforef "Tour du joueur : Joueur 1"))))

(event Custom|RollDiceAndMoveTurnPlayer
  ;[1 0.9472 0.05237] Si la vie été si simple ....
  (bind _result (Default|RollDice (Variables|Default|GetDice)))
  (CallFunction|MovePlayer _result)
  (CallFunction|ChangeTurn))

(event Custom|MovePlayer
  (params (Distance :type Integer))
  (bind _gridref (Variables|Default|GetGridRef))
  (bind _giref (Variables|Default|GetGiRef))
  (bind _playerlist (Variables|/Game/Blueprints/GI_Tabletop.GI_Tabletop_C|GetPlayerList _giref))
  (bind _grid (Variables|/Game/Blueprints/BP_Grid.BP_Grid_C|GetGrid _gridref))
  (bind _turnplayerindex (Variables|/Game/Blueprints/GI_Tabletop.GI_Tabletop_C|GetTurnPlayerIndex _giref))
  (bind _output (Utilities|Array|Get(acopy) _playerlist _turnplayerindex))
  (bind _cell_number (Default|GetPlayerCellNumberbyPlayerId _giref _turnplayerindex))
  (if (< (+ _cell_number Distance) (Utilities|Array|LastIndex _grid))
    (Default|SetPlayerCellNumberbyPlayerId _giref _turnplayerindex (+ _cell_number Distance))
    ;[0.1591 0.3271 1] Super Fonction
    (Default|MovePiontoFirstSlotAvailableinCell (.playerinlevel _output) (Utilities|Array|Get(acopy) (Variables|/Game/Blueprints/BP_Grid.BP_Grid_C|GetGrid (Variables|Default|GetGridRef)) (+ _cell_number Distance)))
    (else
      (CallFunction|Win _turnplayerindex)
      (Default|MovePiontoFirstSlotAvailableinCell (.playerinlevel _output) (Utilities|Array|Get(acopy) _grid (Utilities|Array|LastIndex _grid))))))

(event Custom|Win
  (params (IndexPlayerWhoWon :type Integer))
  (Widget|RemovefromParent (Variables|Default|GetInfoRef))
  (bind _returnvalue (UserInterface|CreateWidget "/Game/Widget/W_Win.W_Win_C"))
  (Variables|/Script/UMG.TextBlock|SetText (Variables|/Game/Widget/W_Win.W_Win_C|GetWinText _returnvalue) (Utilities|Text|ToText(String) (Utilities|String|Append "Bravo Player " (Utilities|String|ToString(Integer) (+ IndexPlayerWhoWon 1)) ", You won !!!")))
  (UserInterface|Viewport|AddtoViewport _returnvalue 0))

(event EventBeginPlay
  (Utilities|FlowControl|Sequence
    (:then_0
      (bind _returnvalue (Actor|GetActorOfClass "/Game/Blueprints/BP_Grid.BP_Grid_C"))
      (Variables|Default|SetGridRef _returnvalue)
      (bind _returnvalue_2 (Game|SpawnActorfromClass "/Game/Blueprints/BP_Dice.BP_Dice_C" (Math|Transform|MakeTransform "0, 0, 0" "0, 0, 0" "1.000000,1.000000,1.000000") "Undefined" "MultiplyWithRoot" 0 0))
      (Variables|Default|SetDice _returnvalue_2))
    (:then_1
      (bind _asgi_tabletop (Utilities|Casting|CastToGI_Tabletop (Game|GetGameInstance))
        (:then
          (Variables|Default|SetGiRef _asgi_tabletop)
          (for (_array_element _array_index) (Variables|/Game/Blueprints/GI_Tabletop.GI_Tabletop_C|GetPlayerList _asgi_tabletop)
            (bind _returnvalue_3 (Game|SpawnActorfromClass "/Game/Blueprints/BP_Player.BP_Player_C" (Math|Transform|MakeTransform "0, 0, 0" "0, 0, 0" "1.000000,1.000000,1.000000") "Undefined" "MultiplyWithRoot" 0 0))
            (Utilities|Array|SetArrayElem (Variables|/Game/Blueprints/GI_Tabletop.GI_Tabletop_C|GetPlayerList _asgi_tabletop) _array_index (Utilities|Struct|MakeStruct_Player (.PlayerNumber (Utilities|Struct|BreakStruct_Player _array_element)) (.Score (Utilities|Struct|BreakStruct_Player _array_element)) (.Position (Utilities|Struct|BreakStruct_Player _array_element)) _returnvalue_3))
            (bind _returnvalue_4 (Game|SpawnActorfromClass "/Game/Blueprints/BP_PionCool.BP_PionCool_C" (Math|Transform|MakeTransform "0.000000,0.000000,85.000000" "0, 0, 0" "1.000000,1.000000,1.000000") "Undefined" "MultiplyWithRoot" 0 0))
            ;[0.002064 0.1104 1] On se souvient de son pion pour plus tard
            (Variables|/Game/Blueprints/BP_Player.BP_Player_C|SetPlayerPion _returnvalue_3 _returnvalue_4)
            ;[0.1591 0.3271 1] Super Fonction
            (Default|MovePiontoFirstSlotAvailableinCell _returnvalue_3 (Utilities|Array|Get(acopy) (Variables|/Game/Blueprints/BP_Grid.BP_Grid_C|GetGrid (Variables|Default|GetGridRef)) (.Position (Utilities|Struct|BreakStruct_Player _array_element))))))
        (:CastFailed
          (Development|PrintString "Mauvais Gi"))))
    (:then_2
      (bind _returnvalue_5 (UserInterface|CreateWidget "/Game/Widget/W_Info.W_Info_C"))
      (bind _output_get (Variables|Default|SetInfoRef _returnvalue_5))
      (UserInterface|Viewport|AddtoViewport _returnvalue_5 0)
      (Default|UpdateScore _output_get))
    (:then_3
      (bind _returnvalue_6 (Actor|GetActorOfClass "/Game/Blueprints/Memory/BP_MemoryGame.BP_MemoryGame_C"))
      (Variables|Default|SetMemoryRef _returnvalue_6)
      (bind _returnvalue_7 (Actor|GetActorOfClass "/Game/Blueprints/Collecte/BP_CollecteManager.BP_CollecteManager_C"))
      (Variables|Default|SetCollecteRef _returnvalue_7))
    (:then_4
      (bind _asbp_player (Utilities|Casting|CastToBP_Player (Game|Player|GetPlayerPawn 0)))
      (Variables|Default|SetDefaultPawn _asbp_player)
      (bind _returnvalue_8 (Actor|GetActorOfClass "/Game/ThirdPerson/Blueprints/BP_ThirdPersonCharacter.BP_ThirdPersonCharacter_C"))
      (Variables|Default|SetCollectPawn _returnvalue_8))))

(fn ConstructionScript)

(fn MoveCameratoBoard
  (Transformation|SetActorTransform (Game|Player|GetPlayerPawn 0) (Utilities|Array|Get(acopy) (Variables|Default|GetCameraPositions))))

(fn MoveCameratoMemory
  (Transformation|SetActorTransform (Game|Player|GetPlayerPawn 0) (Utilities|Array|Get(acopy) (Variables|Default|GetCameraPositions) 1)))

(fn MoveCameratoCollect
  (Transformation|SetActorTransform (Game|Player|GetPlayerPawn 0) (Utilities|Array|Get(acopy) (Variables|Default|GetCameraPositions) 2)))

(fn ShowMemoryWidget
  (bind _inforef (Variables|Default|GetInfoRef))
  (bind _infocollectref (Variables|Default|GetInfoCollectRef))
  (Utilities|IsValid _infocollectref
    (:Is%20Valid
      (Widget|RemovefromParent _infocollectref))
    (:Is%20Not%20Valid
      _))
  (Utilities|IsValid _inforef
    (:Is%20Valid
      (Widget|RemovefromParent _inforef))
    (:Is%20Not%20Valid
      _))
  (Utilities|IsValid (Variables|Default|GetInfoMemoryRef)
    (:Is%20Valid
      _)
    (:Is%20Not%20Valid
      (bind _returnvalue (UserInterface|CreateWidget "/Game/Widget/W_InfoMemory.W_InfoMemory_C"))
      (Variables|Default|SetInfoMemoryRef _returnvalue)))
  (UserInterface|Viewport|AddtoViewport (Variables|Default|GetInfoMemoryRef) 0))

(fn ShowInfoWidget
  (bind _infomemoryref (Variables|Default|GetInfoMemoryRef))
  (bind _infocollectref (Variables|Default|GetInfoCollectRef))
  (Utilities|IsValid _infocollectref
    (:Is%20Valid
      (Widget|RemovefromParent _infocollectref))
    (:Is%20Not%20Valid
      _))
  (Utilities|IsValid _infomemoryref
    (:Is%20Valid
      (Widget|RemovefromParent _infomemoryref))
    (:Is%20Not%20Valid
      _))
  (Utilities|IsValid (Variables|Default|GetInfoRef)
    (:Is%20Valid
      _)
    (:Is%20Not%20Valid
      (bind _returnvalue (UserInterface|CreateWidget "/Game/Widget/W_Info.W_Info_C"))
      (bind _output_get (Variables|Default|SetInfoRef _returnvalue))))
  (UserInterface|Viewport|AddtoViewport (Variables|Default|GetInfoRef) 0)
  (Default|UpdateScore _output_get))

(fn ShowCollectWidget
  (bind _inforef (Variables|Default|GetInfoRef))
  (bind _infomemoryref (Variables|Default|GetInfoMemoryRef))
  (Utilities|IsValid _inforef
    (:Is%20Valid
      (Widget|RemovefromParent _inforef))
    (:Is%20Not%20Valid
      _))
  (Utilities|IsValid _infomemoryref
    (:Is%20Valid
      (Widget|RemovefromParent _infomemoryref))
    (:Is%20Not%20Valid
      _))
  (Utilities|IsValid (Variables|Default|GetInfoCollectRef)
    (:Is%20Valid
      _)
    (:Is%20Not%20Valid
      (bind _returnvalue (UserInterface|CreateWidget "/Game/Widget/W_InfoCollect.W_InfoCollect_C"))
      (Variables|Default|SetInfoCollectRef _returnvalue)))
  (UserInterface|Viewport|AddtoViewport (Variables|Default|GetInfoCollectRef) 0))

(fn SwitchtoCollectPawn
  (bind _collectpawn (Variables|Default|GetCollectPawn))
  (Pawn|Possess (Game|GetPlayerController 0) _collectpawn)
  (Default|InitMieux _collectpawn))

(fn SwitchtoDefaultPawn
  (Pawn|Possess (Game|GetPlayerController 0) (Variables|Default|GetDefaultPawn)))